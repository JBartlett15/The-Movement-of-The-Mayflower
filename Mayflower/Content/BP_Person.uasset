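; BP_Person is an actor representing a named person as a clickable sphere with a text label.
; Sphere cursor events print debug messages: a fixed string on click and the Name variable when hover begins or ends.
; On BeginPlay, a LookAt on the TextRender's relative transform turns the label once toward a hard-coded point, with no per-frame update.
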(event `self.Sphere.OnClicked`
  (params (TouchedComponent :type "PrimitiveComponent Object Reference") (ButtonPressed :type "Key Structure"))
  (`KismetSystemLibrary.PrintString` "Cliked"))

(event `self.Sphere.OnBeginCursorOver`
  (params (TouchedComponent :type "PrimitiveComponent Object Reference"))
  (`KismetSystemLibrary.PrintString` (`self.Name`)))

(event `self.Sphere.OnEndCursorOver`
  (params (TouchedComponent :type "PrimitiveComponent Object Reference"))
  (`KismetSystemLibrary.PrintString` (`self.Name`)))

(event `self.ReceiveBeginPlay`
  (`SceneComponent.K2_SetRelativeTransform` (`self.TextRender`) (`KismetAnimationLibrary.K2_LookAt` (`SceneComponent.GetRelativeTransform` (`self.TextRender`)) (-760.0 -1273.0 1326.0)) false false))

(fn `UserConstructionScript`)