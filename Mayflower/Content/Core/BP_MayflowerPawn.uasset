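; Pawn for a Mayflower game that runs the in-game calendar and shows a day timer HUD.
; On BeginPlay it creates the WBP_DayTimer widget and adds it to the viewport.
; Tick accumulates time while unpaused and, once it reaches a threshold, advances the day and calls CheckDay.
; CheckDay switches on month and day, with only an empty September branch so far.
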(event `self.ReceiveBeginPlay`
  (bind _returnvalue (`|CreateWidget` "/Game/UI/WBP_DayTimer.WBP_DayTimer_C"))
  (bind _output_get (set `self.HUD` _returnvalue))
  (`UserWidget.AddToViewport` _output_get 0))

(event `self.ReceiveTick`
  (params (DeltaSeconds :type "Float (single-precision)"))
  (if (not (`self.TimerPaused`))
    (bind _output_get (set `self.Timer` (+ DeltaSeconds (`self.Timer`))))
    (if (>= _output_get 20.0)
      (`/Engine/EditorBlueprintResources/StandardMacros.IncrementInt` (`self.Day`)
        (:`  `
          (`self.CheckDay`))))))

(event `CheckDay`
  (switch `/Game/Enum_Month` (`self.Month`)
    (:`NewEnumerator0`
      (switch `int` (`self.Day`)))))

(fn `UserConstructionScript`)